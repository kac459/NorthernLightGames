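; IslandBP is a capturable island objective, intended as king-of-the-hill, that changes team ownership.
; When a FirstPersonCharacter from a non-owning team enters the Trigger, it stores that player and starts a CaptureTime timer.
; The timer calls CapturingIsland, which assigns the player's team as owner and recolors CaptureLight red or blue for teams 0 and 1.
; No end-overlap handling exists, so leaving does not cancel capture.
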(event `self.Trigger.OnComponentBeginOverlap`
  (params (OverlappedComponent :type "PrimitiveComponent Object Reference") (OtherActor :type "Actor Object Reference") (OtherComp :type "PrimitiveComponent Object Reference") (OtherBodyIndex :type Integer) (bFromSweep :type Boolean) (SweepResult :type "HitResult Structure (by ref)"))
  ;[1 1 1] Capture Function
  ;;[1 1 1] For now, capture will be KOH style, stand on island for x time
  (bind _asfirst_person_character (cast `/Game/FirstPersonBP/Blueprints/FirstPersonCharacter` OtherActor))
  (bind _output_get (set `self.CapturingPlayer` _asfirst_person_character))
  (if (!= (`/Game/FirstPersonBP/Blueprints/FirstPersonCharacter.TeamNumber` _output_get) (`self.teamOwner`))
    (set `self.isCapturing` true)
    (`KismetSystemLibrary.K2_SetTimer` null "CapturingIsland" (`self.captureTime`))
    (`KismetSystemLibrary.PrintString` "Capturing Island")))

(fn `CapturingIsland`
  (set `self.isCapturing` false)
  (bind _output_get (set `self.teamOwner` (`/Game/FirstPersonBP/Blueprints/FirstPersonCharacter.TeamNumber` (`self.CapturingPlayer`))))
  (`KismetSystemLibrary.PrintString` (`KismetStringLibrary.BuildString_Int` "Island Captured by team" "" _output_get))
  (if (== (`self.teamOwner`) 0)
    (`LightComponent.SetLightColor` (`self.CaptureLight`) (struct :`R` 1.0 :`G` 0.117539 :`A` 1.0) true)
    (elif (== (`self.teamOwner`) 1)
      (`LightComponent.SetLightColor` (`self.CaptureLight`) (struct :`G` 0.177542 :`B` 1.0 :`A` 1.0) true))))

(fn `UserConstructionScript`)